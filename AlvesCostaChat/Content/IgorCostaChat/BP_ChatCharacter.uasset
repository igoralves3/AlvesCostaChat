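; Chat character that links a BP_Chat widget to a socket chat server on localhost.
; BeginPlay spawns a ChatActor as the socket, connects it and shows the widget; EndPlay disconnects.
; SocketSend sends text with a PlayerId-based name and a lobby, private when the lobby field is enabled.
; ReceiveTrue, polled every Tick and bound on send, appends received strings to the dialog once the first send sets Connected.
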(event Custom|SocketConnection
  (Class|ChatActor|Connect (Variables|Default|GetSocket) "127.0.0.1" 5000))

(event Custom|Socket%20Send
  (params (NewParam :type Text))
  (bind _chat (Variables|Default|GetChat))
  (bind _lobbytext (Variables|/Game/IgorCostaChat/BP_Chat.BP_Chat_C|GetLobbyText _chat))
  (if (Variables|Default|Getconnected)
    _
    (else
      (Variables|Default|Setconnected true)
      (Rendering|Components|TextRender|SetText (Variables|/Game/IgorCostaChat/BP_Chat.BP_Chat_C|GetTextAnswer (Variables|Default|GetChat)) "Connected to Chat")))
  (if (> (Utilities|String|Len (Utilities|String|ToString(Text) NewParam)) 0)
    (if (Class|Widget|GetIsEnabled _lobbytext)
      (Variables|Default|SetcurrentLobby (Utilities|String|ToString(Text) (Variables|/Script/UMG.EditableTextBox|GetText _lobbytext)))
      (Variables|Default|Setprivate true)
      (else
        (Variables|Default|SetcurrentLobby "None")
        (Variables|Default|Setprivate false)))
    (Class|ChatActor|SendResurge (Variables|Default|GetSocket) (Utilities|String|ToString(Text) NewParam) (Variables|Default|Getprivate) (Utilities|String|ToString(Text) (Utilities|Text|FormatText "igor {id}" (Variables|/Script/Engine.PlayerState|GetPlayerId (Game|GetPlayerState 0)))) (Variables|Default|GetcurrentLobby))
    (EventDispatchers|BindEventtoOnMessageReceived (Variables|Default|GetSocket) (delegate Custom|ReceiveTrue))))

(event Custom|Socket%20Receive
  (params (Message :type String)))

(event Custom|ReceiveTrue
  (params (Message :type String))
  (bind _chat (Variables|Default|GetChat))
  (bind _dialogtextblock (Variables|/Game/IgorCostaChat/BP_Chat.BP_Chat_C|GetDialogTextBlock _chat))
  (if (Variables|Default|Getconnected)
    (bind _returnvalue (Class|ChatActor|ReceiveDataString (Variables|Default|GetSocket)))
    (if (> (Utilities|String|Len _returnvalue) 0)
      (Development|PrintString (Utilities|String|ToString(Text) (Utilities|Text|ToText(String) _returnvalue)))
      (Rendering|Components|TextRender|SetText _dialogtextblock (Utilities|Text|ToText(String) (Utilities|String|Append (Utilities|String|ToString(Text) (Class|TextBlock|GetText _dialogtextblock)) " 
" (Utilities|String|ToString(Text) (Utilities|Text|ToText(String) _returnvalue))))))))

(event Custom|DeclaraID)

(event EventBeginPlay
  (bind _returnvalue (Game|GetPlayerController 0))
  (bind _returnvalue_2 (Game|SpawnActorfromClass "/Script/AlvesCostaChat.ChatActor" (Transformation|GetActorTransform) "Undefined" "MultiplyWithRoot" 0 0))
  (Variables|Default|SetSocket _returnvalue_2)
  (CallFunction|SocketConnection)
  (bind _returnvalue_3 (UserInterface|CreateWidget "/Game/IgorCostaChat/BP_Chat.BP_Chat_C"))
  (Variables|/Script/Engine.PlayerController|SetbShowMouseCursor _returnvalue true)
  (Input|SetInputModeGameandUI _returnvalue _returnvalue_3 "DoNotLock" true false)
  (bind _output_get (Variables|Default|SetChat _returnvalue_3))
  (UserInterface|Viewport|AddtoViewport _output_get 0)
  (Default|BeginHUD _output_get))

(event EventTick
  (params (DeltaSeconds :type Float%20%28single-precision%29))
  (CallFunction|ReceiveTrue))

(event EventEndPlay
  (params (EndPlayReason :type EEndPlayReason%20Enum :default "Destroyed"))
  (Class|ChatActor|Disconnect (Variables|Default|GetSocket)))

(fn ConstructionScript)

(fn OnRepDialog)

(fn OnRepUserCount)